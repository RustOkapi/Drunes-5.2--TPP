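; HUD Blueprint that creates and manages the main HUD and the pop-up info modal widget.
; On BeginPlay it sets game-only input, displays the main HUD, and registers the info modal in a widget array that it adds to the viewport.
; ToggleWidget makes registered widgets exclusive, showing or collapsing the target and collapsing the rest.
; Hiding the target restores game-only input, while showing it changes only visibility.
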(event EventBeginPlay
  ;[0.03646 0.02791 0.02791] Focus To game
  (Input|SetInputModeGameOnly (Game|GetPlayerController 0) false)
  (Utilities|FlowControl|Sequence
    (:then_0
      ;[0.06771 0.06771 0.06771] Display HUD
      (bind _returnvalue (UserInterface|CreateWidget "/Game/Core/UI/WBP_MainHUD.WBP_MainHUD_C" (Game|GetPlayerController 0)))
      (bind _output_get (Variables|Default|SetHUD _returnvalue))
      (UserInterface|Viewport|AddtoViewport _output_get 0))
    (:then_1
      ;[0.06771 0.06771 0.06771] Info Modals
      (bind _returnvalue_2 (UserInterface|CreateWidget "/Game/Core/UI/WBP_Info_Modals.WBP_Info_Modals_C" (Game|GetPlayerController 0)))
      (bind _output_get_2 (Variables|Default|SetPIck%20Up%20Widgets _returnvalue_2))
      (Utilities|Array|Add (Variables|Default|GetGet%20Widgets) _output_get_2))
    (:then_2
      ;[0.4844 0.4844 0.4844] Add to Viewport
      (for _array_element (Variables|Default|GetGet%20Widgets)
        (UserInterface|Viewport|AddtoViewport _array_element 0)))))

(event Custom|Toggle_Pickup_Widget
  (CallFunction|ToggleWidget (Variables|Default|GetPIck%20Up%20Widgets)))

(fn ConstructionScript)

(fn ToggleWidget
  (params (Target%20Widget :type User%20Widget%20Object%20Reference))
  (Utilities|IsValid Target%20Widget
    (:Is%20Valid
      (Variables|Default|SetWidget%20To%20Focus Target%20Widget)
      (for _array_element (Variables|Default|GetGet%20Widgets)
        (Utilities|IsValid _array_element
          (:Is%20Valid
            (if (== _array_element (Variables|Default|GetWidget%20To%20Focus))
              (if (Widget|IsVisible (Variables|Default|GetWidget%20To%20Focus))
                (CallFunction|FocusGame)
                (else
                  (CallFunction|FocusWidget)))
              (elif (Widget|IsVisible _array_element)
                (Widget|SetVisibility _array_element "Collapsed")))))))))

(fn FocusGame
  (Widget|SetVisibility (Variables|Default|GetWidget%20To%20Focus) "Collapsed")
  (Input|SetInputModeGameOnly (Game|GetPlayerController 0) false))

(fn FocusWidget
  (Widget|SetVisibility (Variables|Default|GetWidget%20To%20Focus) "SelfHitTestInvisible"))