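; C_WeaponFrameWork is an early-stage weapon framework Blueprint that stores a character and camera reference on initialization.
; A separate event starts a fast looping timer and saves its handle, but the Trace event it calls is empty.
; An unconnected debug line trace would cast a short ray forward from the camera and print the hit actor's name.
; Get Default Variables takes a default camera FOV but does nothing with it.
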(event Custom|Trace)

(event Custom|Int%20Trace%20Timer
  (bind _returnvalue (Utilities|Time|SetTimerbyEvent (delegate Custom|Trace) 0.01 true))
  (Variables|Default|SetTrace%20Timer%20Handle _returnvalue))

(event Custom|Init%20WeaponFrameWork
  (params (Charachter :type Base%20Charachter%20Object%20Reference) (Camera :type Camera%20Component%20Object%20Reference))
  ;[0 0 0] Begin Play
  (Variables|Default|SetCharacter Charachter)
  (Variables|Default|SetCamera Camera))