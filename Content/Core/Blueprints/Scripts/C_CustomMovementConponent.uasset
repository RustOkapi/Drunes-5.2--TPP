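; Custom movement component that gives a character vaulting, sliding, sprinting, wall climbing and jump/land feedback.
; Vaulting validates a forward capsule trace for height, slope and clearance, stores the target, then lerps the actor there once VaultEvents runs.
; Sliding adds a floor-aligned impulse unless uphill and lowers friction; wall climbing traces forward and launches the character.
; Tick drives only vault updates; the gated slide and wall-climb updates are disconnected.
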(event Custom|Init%20Custom%20Movement
  (params (Charachter :type Base%20Charachter%20Object%20Reference) (Default%20Walk%20Speed :type Float%20%28double-precision%29))
  ;[1 0.4167 0.4167] Initialize
  (Utilities|GetDefaultVars(Refs) Charachter Default%20Walk%20Speed))

(event EventTick
  (params (DeltaSeconds :type Float%20%28single-precision%29))
  (Variables|Shared|SetDelta%20Seconds DeltaSeconds)
  (Utilities|FlowControl|Sequence
    (:then_1
      (|VaultUpdate))))

(fn CanVault
  (bind (_start _end) (Vaulting|VaultTracePoints 6e+01))
  (bind _character (Variables|Components|GetCharacter))
  (if (Utilities|Enum|Equal(Enum) (Variables|Vaulting|GetVault%20State) "NewEnumerator5")
    (LocalVariables|SetlCapsuleComponent (Variables|/Script/Engine.Character|GetCapsuleComponent _character))
    (bind (_outhit _returnvalue) (Collision|CapsuleTraceByChannel _start _end 25.0 0.0 "TraceTypeQuery1" false (Utilities|Array|MakeArray _character) "None"))
    (if _returnvalue
      (bind (_result _target_location) (Vaulting|CanVaulttoObject (LocalVariables|GetlCapsuleComponent) _outhit))
      (return _result _target_location)
      (else
        (return false "0, 0, 0")))
    (else
      (return false "0, 0, 0"))))

(fn VaultTracePoints
  (params (Length :type Float%20%28single-precision%29))
  (bind _returnvalue (Utilities|GetCapsuleHalfHeight))
  (bind _character (Variables|Components|GetCharacter))
  (bind _returnvalue_2 (Transformation|GetActorLocation _character))
  (bind _returnvalue_3 (Transformation|GetActorForwardVector _character))
  (bind _returnvalue_4 (* _returnvalue_3 Length))
  (bind _returnvalue_5 (+ _returnvalue_2 _returnvalue_4))
  (return (+ _returnvalue_5 (Math|Vector|MakeVector 0.0 0.0 _returnvalue)) (- _returnvalue_5 (Math|Vector|MakeVector 0.0 0.0 _returnvalue))))

(fn CanVaulttoObject
  (params (Capsule :type Capsule%20Component%20Object%20Reference) (Hit :type Hit%20Result%20Structure))
  (bind _character (Variables|Components|GetCharacter))
  (bind _capsulecomponent (Variables|/Script/Engine.Character|GetCapsuleComponent _character))
  (bind _returnvalue (Components|Capsule|GetScaledCapsuleRadius _capsulecomponent))
  (bind _returnvalue_2 (Components|Capsule|GetScaledCapsuleHalfHeight _capsulecomponent))
  (Utilities|FlowControl|Sequence
    (:then_0
      ;[1 1 1] Is Valid Height
      (if (not (Math|Float|InRange(Float) (- (.Z (Math|Vector|BreakVector (.location Hit))) (.Z (Math|Vector|BreakVector (.traceend Hit)))) (Variables|Vaulting|GetMin%20Vault%20Height) (Variables|Vaulting|GetMax%20Vault%20Height)))
        (return false "0, 0, 0")))
    (:then_1
      ;[1 1 1] Valid Walkable Steepness
      (if (< (.Z (Math|Vector|BreakVector (.normal Hit))) (Class|CharacterMovementComponent|GetWalkableFloorZ (Variables|/Script/Engine.Character|GetCharacterMovement (Variables|Components|GetCharacter))))
        (return false "0, 0, 0")))
    (:then_2
      ;[1 1 1] Does Have Enough Room To Vault
      (bind _output_get (LocalVariables|SetlTargetLocation (+ (.location Hit) (Math|Vector|MakeVector 0.0 0.0 _returnvalue_2))))
      (bind _result_ (Vaulting|CheckVaultCapsuleCollision false (+ _output_get (Math|Vector|MakeVector 0.0 0.0 _returnvalue)) _returnvalue_2 _returnvalue))
      (if _result_
        (return false "0, 0, 0")))
    (:then_3
      (return true (LocalVariables|GetlTargetLocation)))))

(fn CheckVaultCapsuleCollision
  (params (Draw%20Debug :type Boolean) (Centre :type Vector) (Half%20Height :type Float%20%28double-precision%29) (Radius :type Float%20%28double-precision%29))
  (Utilities|FlowControl|Sequence
    (:then_0
      (if Draw%20Debug
        (Rendering|Debug|DrawDebugCapsule Centre Half%20Height Radius "0, 0, 0" "(R=1.000000,G=1.000000,B=1.000000,A=1.000000)" 0.0 3.0)))
    (:then_1
      (bind _returnvalue (Collision|CapsuleOverlapActors Centre Radius Half%20Height (Utilities|Array|MakeArray "ObjectTypeQuery1" "ObjectTypeQuery2" "ObjectTypeQuery1" "ObjectTypeQuery4") 0 (Utilities|Array|MakeArray (Variables|Components|GetCharacter))))
      (return _returnvalue))))

(fn TickVault
  (params (Delta%20Seconds :type Float%20%28double-precision%29))
  (Utilities|FlowControl|Sequence
    (:then_0
      (Variables|Shared|SetAlpha (Math|Float|Clamp(Float) (+ (Variables|Shared|GetAlpha) (/ Delta%20Seconds (Variables|Vaulting|Get%20Vault%20Time)))))
      (Transformation|SetActorLocation (Variables|Components|GetCharacter) (Math|Vector|Lerp(Vector) (Variables|Vaulting|GetStarting%20Location%20V) (Variables|Vaulting|GetTarget%20Location%20V) (Variables|Shared|GetAlpha)) false false))
    (:then_1
      (if (>= (Variables|Shared|GetAlpha) 1.0)
        (Variables|Vaulting|SetVault%20State "NewEnumerator5")))))

(fn CanSlide
  (if (and (Utilities|Enum|Equal(Enum) (Variables|Slide|GetSlideState) "NewEnumerator8") (Utilities|Enum|Equal(Enum) (Variables|Sprint|GetSprint%20State) "NewEnumerator0"))
    (if (and (> (CallFunction|GetForwardInput) 0.0) (not (AI|Components|NavMovement|IsFalling (Variables|/Script/Engine.Character|GetCharacterMovement (Variables|Components|GetCharacter)))))
      (return true)
      (else
        (return false)))))

(fn GetForwardInput
  (return (Math|Vector|DotProduct (Transformation|GetActorForwardVector (Variables|Components|GetCharacter)) (Pawn|Components|PawnMovement|GetLastInputVector (Variables|/Script/Engine.Character|GetCharacterMovement (Variables|Components|GetCharacter))))))

(fn GetWallTracePoints
  (return (+ (+ (.OutLocation (Actor|GetActorEyesViewPoint (Variables|Components|GetCharacter))) "") (* (Transformation|GetActorForwardVector (Variables|Components|GetCharacter)) 35.0)) (+ (- (Transformation|GetActorLocation (Variables|Components|GetCharacter)) (Math|Vector|MakeVector 0.0 0.0 (Variables|/Script/Engine.CapsuleComponent|GetCapsuleHalfHeight (Variables|/Script/Engine.Character|GetCapsuleComponent (Variables|Components|GetCharacter))))) (* (Transformation|GetActorForwardVector (Variables|Components|GetCharacter)) 5e+01))))

(fn SlideStart
  (bind _returnvalue (Utilities|SlideVector))
  (bind _character (Variables|Components|GetCharacter))
  (bind _result (Slide|CanSlide))
  (if _result
    (CallFunction|OpenSlideCheckGate)
    (Character|Crouch _character)
    (Utilities|ValidSlope? _returnvalue
      (:true
        (Physics|AddImpulse (Variables|/Script/Engine.Character|GetCharacterMovement _character) (* _returnvalue (Variables|Slide|GetSlide%20Impulse)) true)
        (Utilities|SetSlideVariables 0.0 1.4e+03 "NewEnumerator7")))))

(fn SlideEnd
  (if (Variables|/Game/Core/Blueprints/Base_Charachter.Base_Charachter_C|GetbHoldingCrouch (Variables|Components|GetCharacter))
    (Character|Crouch (Variables|Components|GetCharacter))
    (else
      (Character|UnCrouch (Variables|Components|GetCharacter))))
  (Utilities|SetSlideVariables 8.0 4096.0 "NewEnumerator8")
  (CallFunction|CloseSlideCheckGate))

(fn PlayCameraShake
  (params (Shake :type Camera%20Shake%20Base%20Class%20Reference))
  (if (Variables|Default|GetShake%20Camera?)
    (Camera|PlayWorldCameraShake Shake (Transformation|GetWorldLocation (Variables|/Game/Core/Blueprints/Base_Charachter.Base_Charachter_C|GetCamera (Variables|Components|GetCharacter))) 0.0 1e+02)))

(fn SprintStart
  (Variables|Sprint|SetSprint%20State "NewEnumerator0")
  (Variables|/Script/Engine.CharacterMovementComponent|SetMaxWalkSpeed (Variables|/Script/Engine.Character|GetCharacterMovement (Variables|Components|GetCharacter)) (Math|Interpolation|FInterpTo (Variables|Sprint|GetDefault%20Walk%20Speed) (Variables|Sprint|GetSprint%20Speed) (Variables|Shared|GetDelta%20Seconds) 6e+01)))

(fn SprintEnd
  (Variables|Sprint|SetSprint%20State "NewEnumerator2")
  (Variables|/Script/Engine.CharacterMovementComponent|SetMaxWalkSpeed (Variables|/Script/Engine.Character|GetCharacterMovement (Variables|Components|GetCharacter)) (Math|Interpolation|FInterpTo (Variables|Sprint|GetSprint%20Speed) (Variables|Sprint|GetDefault%20Walk%20Speed) (Variables|Shared|GetDelta%20Seconds) 4e+01)))

(fn JumpEvents
  (Character|Jump (Variables|Components|GetCharacter))
  (CallFunction|OpenWallClimbGate)
  (CallFunction|PlayCameraShake "/Game/Core/Blueprints/Player-Data/Camera_Shake/CameraShakes/CameraShake_Jump_Soft.CameraShake_Jump_Soft_C")
  (Audio|PlaySound2D "/Game/Core/Assets/Audio/JUMPs/SC_Jump_Concrete.SC_Jump_Concrete" 1.0 1.0 0.0 0 0))

(fn LandEvents
  (CallFunction|CloseWallClimbGate)
  (if (> (Utilities|GetVelocity) (Variables|FallDamage|GetMax%20Safe%20Falling%20Velocity))
    (CallFunction|PlayCameraShake "/Game/Core/Blueprints/Player-Data/Camera_Shake/CameraShakes/CameraShake_Land_Soft.CameraShake_Land_Soft_C")
    (else
      (CallFunction|PlayCameraShake "/Game/Core/Blueprints/Player-Data/Camera_Shake/CameraShakes/CameraShake_Jump_Soft.CameraShake_Jump_Soft_C")))
  (if (and (> (Utilities|GetVelocity) 4e+02) (Utilities|Enum|Equal(Enum) (Variables|Vaulting|GetVault%20State) "NewEnumerator5"))
    (Audio|PlaySound2D "/Game/Core/Assets/Audio/LANDs/SC_Land_Concrete.SC_Land_Concrete" 1.0 1.0 0.0 0 0)))

(fn VaultEvents
  (bind _character (Variables|Components|GetCharacter))
  (bind _charactermovement (Variables|/Script/Engine.Character|GetCharacterMovement _character))
  (Utilities|SetVaultingVars)
  (if (Utilities|Enum|Equal(Enum) (Variables|LedgeGrab|GetLedge%20Grab%20State) "NewEnumerator4")
    (Pawn|Components|CharacterMovement|SetMovementMode _charactermovement "MOVE_Walking" 0)
    (Variables|/Script/Engine.CharacterMovementComponent|SetGravityScale _charactermovement 1.4)
    (Variables|LedgeGrab|SetLedge%20Grab%20State "NewEnumerator5")))

(fn CanWallClimb
  (return (Math|Boolean|ANDBoolean (> (CallFunction|GetForwardInput) 0.0) (AI|Components|NavMovement|IsFalling (Variables|/Script/Engine.Character|GetCharacterMovement (Variables|Components|GetCharacter))) (Utilities|Enum|Equal(Enum) (Variables|Vaulting|GetVault%20State) "NewEnumerator5") (Utilities|Enum|Equal(Enum) (Variables|Slide|GetSlideState) "NewEnumerator8"))))

(fn WallClimbUpdate
  (bind _feet_location (WallClimb|GetWallTracePoints))
  (if (WallClimb|CanWallClimb)
    (bind _can_vault_ (Vaulting|CanVault))
    (if (not _can_vault_)
      (bind (_outhit _returnvalue) (Collision|LineTraceByChannel _feet_location (+ _feet_location (* (Transformation|GetActorForwardVector (Variables|Components|GetCharacter)) 5e+01)) "TraceTypeQuery1" false 0 "None" true "(R=1.000000,G=0.000000,B=0.000000,A=1.000000)" "(R=0.000000,G=1.000000,B=0.000000,A=1.000000)" 35.0))
      (if (and (> (CallFunction|GetForwardInput) 0.0) _returnvalue)
        (Variables|WallClimb|SetWall%20Climb%20Normal (.ImpactNormal (Collision|BreakHitResult _outhit)))
        (Character|LaunchCharacter (Variables|Components|GetCharacter) (Math|Vector|MakeVector (.x (* (Variables|WallClimb|GetWall%20Climb%20Normal) -6e+02)) (.y (* (Variables|WallClimb|GetWall%20Climb%20Normal) -6e+02)) (Variables|WallClimb|GetWall%20Climb%20Speed)) true true)))))

(fn WallClimbEnd
  (CallFunction|CloseWallClimbGate))

(fn WallClimbStart)

(event Custom|Close%20Slide%20Check%20Gate
  (Utilities|FlowControl|Gate true) ; enters at Close
)

(event Custom|Open%20Slide%20Check%20Gate
  (Utilities|FlowControl|Gate true) ; enters at Open
)

(event Custom|Close%20Wall%20Climb%20Gate
  (Utilities|FlowControl|Gate true) ; enters at Close
)

(event Custom|Open%20Wall%20Climb%20Gate
  (Utilities|FlowControl|Gate true) ; enters at Open
)