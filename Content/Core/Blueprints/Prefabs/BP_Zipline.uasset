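; BP_Zipline is a zipline prefab that draws its line with a Cable component laid along a Spline.
; ConstructCable moves the cable to the first spline point, attaches its end at the second point's local position and matches its length to the spline length.
; The construction script and SetTransform are empty, and the file shows neither a call to ConstructCable nor any riding logic.
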(fn ConstructionScript)

(fn ConstructCable
  (Transformation|SetWorldLocation (Variables|Default|GetCable) (Spline|GetLocationatSplinePoint (Variables|Default|GetSpline) 0 "World") false false)
  (Variables|/Script/CableComponent.CableComponent|SetbAttachEnd (Variables|Default|GetCable) true)
  (Variables|/Script/CableComponent.CableComponent|SetEndLocation (Variables|Default|GetCable) (Spline|GetLocationatSplinePoint (Variables|Default|GetSpline) 1 "Local"))
  (Variables|/Script/CableComponent.CableComponent|SetCableLength (Variables|Default|GetCable) (Spline|GetSplineLength (Variables|Default|GetSpline))))

(fn SetTransform)