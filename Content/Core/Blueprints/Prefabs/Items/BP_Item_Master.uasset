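; BP_Item_Master is the base item Blueprint, providing the pickup prompt shown when a Character enters its sphere.
; BeginPlay caches player 0's HUD_CoreWidget; sphere begin overlap toggles its pickup widget and sets the text to "E" plus ItemPickupText.
; End overlap toggles the widget again for any actor, without the Character check.
; ItemPickupText returns only base-item placeholder text, and no pickup input is handled here.
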(event OnComponentBeginOverlap(Sphere)
  (params (OverlappedComponent :type Primitive%20Component%20Object%20Reference) (OtherActor :type Actor%20Object%20Reference) (OtherComp :type Primitive%20Component%20Object%20Reference) (OtherBodyIndex :type Integer) (bFromSweep :type Boolean) (SweepResult :type Hit%20Result%20Structure%20%28by%20ref%29))
  (bind _core_hud (Variables|Default|GetCore_HUD))
  (Utilities|Casting|CastToCharacter OtherActor)
  (Default|TogglePickupWidget _core_hud)
  (Default|SetText (Variables|/Game/Core/Blueprints/FrameWork/HUD_CoreWidget.HUD_CoreWidget_C|GetPIck%20Up%20Widgets _core_hud) (Utilities|Text|FormatText "E  {name}" (CallFunction|ItemPickupText))))

(event OnComponentEndOverlap(Sphere)
  (params (OverlappedComponent :type Primitive%20Component%20Object%20Reference) (OtherActor :type Actor%20Object%20Reference) (OtherComp :type Primitive%20Component%20Object%20Reference) (OtherBodyIndex :type Integer))
  (Default|TogglePickupWidget (Variables|Default|GetCore_HUD)))

(event EventBeginPlay
  (bind _ashud_core_widget (Utilities|Casting|CastToHUD_CoreWidget (HUD|GetHUD (Game|GetPlayerController 0))))
  (Variables|Default|SetCore_HUD _ashud_core_widget))

(fn ConstructionScript)

(fn ItemPickupText
  (return "There Is No Fucking Item here Dickhead !! Its The Fucking Base Item"))